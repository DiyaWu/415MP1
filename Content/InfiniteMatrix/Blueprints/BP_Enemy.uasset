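; Enemy actor that damages the player on contact and awards score when shot.
; A hit on BP_Player shakes the camera and removes one health, then either flags death and shows restart at zero health or destroys the enemy.
; Overlap with a BP_Shooting actor destroys both and increments the player's score.
; The player overlapping TriggerZone destroys the enemy without changing score or health.
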(event OnComponentHit(Enemy)
  (params (HitComponent :type Primitive%20Component%20Object%20Reference) (OtherActor :type Actor%20Object%20Reference) (OtherComp :type Primitive%20Component%20Object%20Reference) (NormalImpulse :type Vector :default "0, 0, 0") (Hit :type Hit%20Result%20Structure%20%28by%20ref%29))
  (bind _asbp_player (Utilities|Casting|CastToBP_Player OtherActor))
  (Camera|PlayWorldCameraShake "/Game/InfiniteMatrix/Blueprints/correctShake.BP_Shake_C" (Transformation|GetActorLocation _asbp_player) 0.0 5e+02)
  (bind _output_get (Variables|/Game/InfiniteMatrix/Blueprints/BP_Player.BP_Player_C|SetHealth _asbp_player (- (Variables|/Game/InfiniteMatrix/Blueprints/BP_Player.BP_Player_C|GetHealth _asbp_player) 1)))
  (if (<= _output_get 0)
    (Variables|/Game/InfiniteMatrix/Blueprints/BP_Player.BP_Player_C|SetIsDead _asbp_player true)
    (Default|DisplayRestart _asbp_player)
    (else
      (Actor|DestroyActor))))

(event OnComponentBeginOverlap(triggerZone)
  (params (OverlappedComponent :type Primitive%20Component%20Object%20Reference) (OtherActor :type Actor%20Object%20Reference) (OtherComp :type Primitive%20Component%20Object%20Reference) (OtherBodyIndex :type Integer) (bFromSweep :type Boolean) (SweepResult :type Hit%20Result%20Structure%20%28by%20ref%29))
  (Utilities|Casting|CastToBP_Player OtherActor)
  (Actor|DestroyActor))

(event OnComponentBeginOverlap(Enemy)
  (params (OverlappedComponent :type Primitive%20Component%20Object%20Reference) (OtherActor :type Actor%20Object%20Reference) (OtherComp :type Primitive%20Component%20Object%20Reference) (OtherBodyIndex :type Integer) (bFromSweep :type Boolean) (SweepResult :type Hit%20Result%20Structure%20%28by%20ref%29))
  (bind _asbp_shooting (Utilities|Casting|CastToBP_Shooting OtherActor))
  (Actor|DestroyActor)
  (Actor|DestroyActor _asbp_shooting)
  (bind _returnvalue (Actor|GetActorOfClass "/Game/InfiniteMatrix/Blueprints/BP_Player.BP_Player_C"))
  (Variables|/Game/InfiniteMatrix/Blueprints/BP_Player.BP_Player_C|SetScore _returnvalue (+ (Variables|/Game/InfiniteMatrix/Blueprints/BP_Player.BP_Player_C|GetScore _returnvalue) 1)))

(event EventBeginPlay)

(event Collision|EventActorBeginOverlap
  (params (OtherActor :type Actor%20Object%20Reference)))

(event EventTick
  (params (DeltaSeconds :type Float%20%28single-precision%29)))

(fn ConstructionScript)